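; BPThirdCharacter is a player character that moves, aims with the mouse and fires a gun.
; On BeginPlay it spawns a BPGun at Arrow1 and attaches it to the mesh, with left click driving its trigger.
; Each tick, a cursor trace gives an aim direction, and the arcsine of its flattened dot with mesh forward adjusts mesh yaw.
; The mouse wheel zooms the spring arm, and EffectHealth recalculates and prints health.
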(event `self.ReceiveBeginPlay`
  (bind _returnvalue (`|SpawnActorFromClass` "/Game/Blueprint/BPGun.BPGun_C" (`SceneComponent.K2_GetComponentToWorld` (`self.Arrow1`)) "Undefined" "OverrideRootScale" null "/Game/Blueprint/Projectile.Projectile_C" null))
  (bind _output_get (set `self.Gun` _returnvalue))
  (`self.K2_AttachToComponent` _output_get (`self.Mesh`) "None" "KeepWorld" "KeepWorld" "KeepWorld" true))

(event `Key|MouseScrollUp`
  (params (Key :type "Key Structure"))
  (bind _springarm (`self.SpringArm`))
  (bind _targetarmlength (`SpringArmComponent.TargetArmLength` _springarm))
  ;[1 1 1] 控制视野gaodi
  (:`Pressed`
    (if (>= _targetarmlength 200.0)
      (set `SpringArmComponent.TargetArmLength` (- _targetarmlength 20.0) _springarm))))

(event `Key|MouseScrollDown`
  (params (Key :type "Key Structure"))
  (bind _springarm (`self.SpringArm`))
  (bind _targetarmlength (`SpringArmComponent.TargetArmLength` _springarm))
  ;[1 1 1] 控制视野gaodi
  (:`Pressed`
    (if (<= _targetarmlength 900.0)
      (set `SpringArmComponent.TargetArmLength` (+ _targetarmlength 20.0) _springarm))))

(event `Key|LeftMouseButton`
  (params (Key :type "Key Structure"))
  (bind _gun (`self.Gun`))
  (:`Pressed`
    (`/Game/Blueprint/BPGun.PullTigger` _gun))
  (:`Released`
    (`/Game/Blueprint/BPGun.ReleaseTigger` _gun)))

(event `InputAxis|MoveForward`
  (params (AxisValue :type "Float (single-precision)"))
  ;[1 1 1] 控制移动
  (`self.AddMovementInput` (`self.GetActorForwardVector`) AxisValue))

(event `self.ReceiveEndPlay`
  (params (EndPlayReason :type "EEndPlayReason Enum" :default "Destroyed"))
  (`self.K2_DestroyActor` (`self.Gun`)))

(event `InputAxis|MoveRight`
  (params (AxisValue :type "Float (single-precision)"))
  ;[1 1 1] 控制移动
  (`self.AddMovementInput` (`self.GetActorRightVector`) AxisValue))

(event `self.ReceiveTick`
  (params (DeltaSeconds :type "Float (single-precision)"))
  ;[1 1 1] 人物向鼠标方向旋转
  (bind _location (`self.GetMpuseToPersonVector`)
    (:`out`
      (`self.MakesureRotate` _location (`SceneComponent.GetForwardVector` (`self.Mesh`))))))

(event `/Game/Blueprint/fireinterface.EffectHealth`
  (params (Delta :type "Float (single-precision)"))
  ;[1 1 1] 人物gg
  (`self.CalculateHealth` Delta)
  (`KismetSystemLibrary.PrintString` (`KismetStringLibrary.Conv_DoubleToString` (`self.Health`))))

(fn `UserConstructionScript`)