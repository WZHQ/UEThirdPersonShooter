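; An enemy spawner actor that keeps spawning BPThirdAI pawns at random points inside its Box volume while the ThirdCharacter count stays below ten.
; BeginPlay starts two looping timers: a fast one attempts spawns, and a slower one raises Level over time.
; Tick recounts all ThirdCharacter actors every frame to feed the population cap.
; Each new pawn receives the current Level as EnemyLevel, so later spawns carry higher levels.
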(event `self.ReceiveBeginPlay`
  (`KismetSystemLibrary.K2_SetTimerDelegate` (delegate `SpawnEnemy`) 1.0 true)
  (`KismetSystemLibrary.K2_SetTimerDelegate` (delegate `addtime`) 15.0 true))

(event `self.ReceiveTick`
  (params (DeltaSeconds :type "Float (single-precision)"))
  (bind _outactors (`GameplayStatics.GetAllActorsOfClass` "/Script/ThirdShootGame.ThirdCharacter"))
  (set `self.EnemyNumber` (`KismetArrayLibrary.Array_Length` _outactors)))

(event `addtime`
  (set `self.level` (+ (`self.level`) 1)))

(event `SpawnEnemy`
  (if (<= (`self.EnemyNumber`) 9)
    (bind _returnvalue (`AIBlueprintHelperLibrary.SpawnAIFromClass` "/Game/Blueprint/BPThirdAI.BPThirdAI_C" null (`KismetMathLibrary.RandomPointInBoundingBox` (`self.K2_GetActorLocation`) (`BoxComponent.BoxExtent` (`self.Box`)))))
    (bind _output_get (set `self.pawn` _returnvalue))
    (bind _asbpthird_ai (cast `/Game/Blueprint/BPThirdAI` _output_get))
    (set `/Game/Blueprint/BPThirdAI.EnemyLevel` (`self.level`) _asbpthird_ai)))

(fn `UserConstructionScript`)