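; BPGun is a gun Blueprint that fires automatically while its trigger is held.
; PullTigger passes through a DoOnce, fires at once, then starts a looping Fire timer with a randomized rate chosen per pull.
; Fire spawns a Bullet at the Arrow component's world transform, and ReleaseTigger clears the timer and resets the DoOnce.
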(event `PullTigger`
  (`/Engine/EditorBlueprintResources/StandardMacros.DoOnce` false :!label _label
    (:`Completed`
      (`self.Fire`)
      (`KismetSystemLibrary.K2_SetTimer` null "Fire" (/ 1.0 (`KismetMathLibrary.RandomFloatInRange` 3.0 10.0)) true))))

(event `ReleaseTigger`
  (`KismetSystemLibrary.K2_ClearTimer` null "Fire")
  (goto _label :!via `Reset`))

(event `Fire`
  (`|SpawnActorFromClass` (`self.bullet`) (`SceneComponent.K2_GetComponentToWorld` (`self.Arrow`)) "Undefined" "OverrideRootScale" null null))

(fn `UserConstructionScript`)