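; AI controller for a BPThirdAI enemy that chases the first player's pawn and shoots on arrival.
; On BeginPlay it caches the controlled pawn and starts a looping timer that re-issues an AIMoveTo toward the player every two seconds.
; The pawn's IsCanWalk flag is cleared before each move and set on success, then after a short delay its gun trigger is pulled and immediately released.
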(event `self.ReceiveBeginPlay`
  (bind _asbpthird_ai (cast `/Game/Blueprint/BPThirdAI` (`self.K2_GetPawn`)))
  (set `self.Enemy` _asbpthird_ai)
  (`KismetSystemLibrary.K2_SetTimerDelegate` (delegate `FollowingHero`) 2.0 true))

(event `FollowingHero`
  (bind _returnvalue (`GameplayStatics.GetPlayerPawn` 0))
  (bind _gun (`/Game/Blueprint/BPThirdAI.Gun` (`self.Enemy`)))
  (set `/Game/Blueprint/BPThirdAI.isCanWalk` false (`self.Enemy`))
  (`/Engine/EditorBlueprintResources/StandardMacros.IsValid` _returnvalue
    (:`Is Valid`
      (`|AIMoveTo` (`self.K2_GetPawn`) (0.0 0.0 0.0) _returnvalue 400.0 true
        (:`OnSuccess`
          (set `/Game/Blueprint/BPThirdAI.isCanWalk` true (`self.Enemy`))
          (`KismetSystemLibrary.Delay` 0.5)
          (`/Game/Blueprint/BPGun.PullTigger` _gun)
          (`/Game/Blueprint/BPGun.ReleaseTigger` _gun))))))

(fn `UserConstructionScript`)