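; Game mode for a third-person shooter that respawns the player character after death.
; On BeginPlay it caches the player pawn as a BPThirdCharacter.
; Tick polls that pawn's IsDead flag, destroys it when set, and after a short delay spawns a replacement at the death transform and possesses it with the first player controller.
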(event `self.ReceiveBeginPlay`
  (bind _asbpthird_character (cast `/Game/Blueprint/BPThirdCharacter` (`GameplayStatics.GetPlayerPawn` 0)))
  (set `self.Pawn` _asbpthird_character))

(event `self.ReceiveTick`
  (params (DeltaSeconds :type "Float (single-precision)"))
  (bind _pawn (`self.Pawn`))
  (`/Engine/EditorBlueprintResources/StandardMacros.IsValid` _pawn
    (:`Is Valid`
      (if (`ThirdCharacter.isDead` _pawn)
        (set `self.transform` (`self.GetTransform` _pawn))
        (`self.K2_DestroyActor` (`self.Pawn`))
        (`KismetSystemLibrary.Delay` 5.0)
        (bind _returnvalue (`|SpawnActorFromClass` "/Game/Blueprint/BPThirdCharacter.BPThirdCharacter_C" (`self.transform`) "Undefined" "OverrideRootScale" null null))
        (bind _output_get (set `self.Pawn` _returnvalue))
        (`Controller.Possess` (`GameplayStatics.GetPlayerController` 0) _output_get)))))

(fn `UserConstructionScript`)