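; BPThirdAI is an armed enemy character whose body color, gun color and health scale with EnemyLevel.
; On BeginPlay it tints dynamic materials and attaches a spawned BPGun to the UseGun socket.
; Tick yaws the mesh toward the player via a flattened dot-product arcsine while IsCanWalk, otherwise resetting its rotation.
; EffectHealth applies health changes; on death it disables collision, then destroys itself and the gun after a delay.
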(event `self.ReceiveBeginPlay`
  (bind _output (`|GetArrayItem` (`self.color`) (`self.EnemyLevel`)))
  (`MaterialInstanceDynamic.SetVectorParameterValue` (`self.charactercolor`) "BodyColor" _output)
  (`MaterialInstanceDynamic.SetVectorParameterValue` (`self.GunColor`) "BodyColor" _output)
  (set `self.Health` (* (`self.EnemyLevel`) 100.0))
  (bind _returnvalue (`|SpawnActorFromClass` "/Game/Blueprint/BPGun.BPGun_C" (`SceneComponent.K2_GetComponentToWorld` (`self.Mesh`)) "Undefined" "OverrideRootScale" null "/Game/Blueprint/AnrmyProjectile.AnrmyProjectile_C" null))
  (bind _output_get (set `self.Gun` _returnvalue))
  (`self.K2_AttachToComponent` _output_get (`self.Mesh`) "UseGun" "SnapToTarget" "SnapToTarget" "SnapToTarget" true)
  (`PrimitiveComponent.SetMaterial` (`/Game/Blueprint/BPGun.SkeletalMesh` (`self.Gun`)) 0 (`self.GunColor`)))

(event `/Game/Blueprint/fireinterface.EffectHealth`
  (params (Delta :type "Float (single-precision)"))
  (`self.CalculateHealth` Delta)
  (`KismetSystemLibrary.PrintString` (`KismetStringLibrary.Conv_DoubleToString` (`self.Health`)))
  (if (`self.isDead`)
    (`PrimitiveComponent.SetCollisionEnabled` (`self.CapsuleComponent`) "NoCollision")
    (`PrimitiveComponent.SetCollisionEnabled` (`self.Mesh`) "NoCollision")
    (`PrimitiveComponent.SetCollisionEnabled` (`/Game/Blueprint/BPGun.SkeletalMesh` (`self.Gun`)) "NoCollision")
    (`KismetSystemLibrary.Delay` 1.9)
    (`self.K2_DestroyActor`)
    (`self.K2_DestroyActor` (`self.Gun`))))

(event `self.ReceiveTick`
  (params (DeltaSeconds :type "Float (single-precision)"))
  (bind _asthird_character (cast `ThirdCharacter` (`GameplayStatics.GetPlayerPawn` 0)))
  (bind _output_get (set `self.Hero` _asthird_character))
  (`/Engine/EditorBlueprintResources/StandardMacros.IsValid` _output_get
    (:`Is Valid`
      (if (`self.isDead`)
        _
        (elif (`self.isCanWalk`)
          (`self.RotateToHero` (`SceneComponent.GetForwardVector` (`self.Mesh`)) (- (`SceneComponent.K2_GetComponentLocation` (`Character.Mesh` (`self.Hero`))) (`SceneComponent.K2_GetComponentLocation` (`self.Mesh`))))
          (else
            (`SceneComponent.K2_SetRelativeRotation` (`self.Mesh`) (struct :`Yaw` -90.0) false false)))))))

(fn `RotateToHero`
  (params (old :type "Vector Structure") (new :type "Vector Structure"))
  (`SceneComponent.K2_SetWorldRotation` (`self.Mesh`) (`KismetMathLibrary.MakeRotator` (.roll (`SceneComponent.K2_GetComponentRotation` (`self.Mesh`))) (.pitch (`SceneComponent.K2_GetComponentRotation` (`self.Mesh`))) (- (.yaw (`SceneComponent.K2_GetComponentRotation` (`self.Mesh`))) (`KismetMathLibrary.DegAsin` (`KismetMathLibrary.Dot_VectorVector` (`KismetMathLibrary.MakeVector` (.x (`KismetMathLibrary.Normal` old)) (.y (`KismetMathLibrary.Normal` old))) (`KismetMathLibrary.MakeVector` (.x (`KismetMathLibrary.Normal` new)) (.y (`KismetMathLibrary.Normal` new))))))) false false))

(fn `UserConstructionScript`
  (bind _returnvalue (`PrimitiveComponent.CreateDynamicMaterialInstance` (`self.Mesh`) 0 "/Game/AnimationAssets/UE4_Mannequin/Materials/M_UE4Man_Body.M_UE4Man_Body"))
  (set `self.charactercolor` _returnvalue)
  (bind _returnvalue_2 (`KismetMaterialLibrary.CreateDynamicMaterialInstance` "/Game/FPWeapon/Materials/MI_FPGun.MI_FPGun"))
  (set `self.GunColor` _returnvalue_2))