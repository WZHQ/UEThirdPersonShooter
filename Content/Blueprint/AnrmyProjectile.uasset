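; Projectile actor, apparently fired by enemies, that affects the health of actors tagged as friendly.
; On overlap, it checks for Fireinterface and the "isfirendly" tag, sends a fixed EffectHealthMessage to matches, then destroys itself.
; Overlapping an actor without the interface also destroys it, while implementers lacking the tag are ignored.
; The construction script tints ProjectileMat blue through its color parameter.
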(event `self.ReceiveActorBeginOverlap`
  (params (OtherActor :type "Actor Object Reference"))
  (if (`KismetSystemLibrary.DoesImplementInterface` OtherActor "/Game/Blueprint/fireinterface.fireinterface_C")
    (if (`self.ActorHasTag` OtherActor "isfirendly")
      (message `/Game/Blueprint/fireinterface.EffectHealth` OtherActor 5.0)
      (`self.K2_DestroyActor` :!label _label))
    (else
      (goto _label))))

(fn `UserConstructionScript`
  (`parent.UserConstructionScript`)
  (`MaterialInstanceDynamic.SetVectorParameterValue` (`self.ProjectileMat`) "color" (struct :`B` 1.0 :`A` 1.0)))